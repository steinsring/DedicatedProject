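; Player controller for the Sci-fi UI Pack that drives its menus, gameplay HUD and demo inputs.
; BeginPlay opens either the multiplayer lobby or a timed loading screen followed by the start screen.
; Home, single-player and multiplayer stack widgets receive pushed activatable menus, submenus and dialogs, with input mode switched between UI and game.
; Input events trigger weapon and skill HUD calls, adjust clamped health and energy, and focus chat.
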(event `self.Open Inventory `
  ;[0.0625 0.01759 0 0.833 45] Open Inventory menu
  (bind _returnvalue (`|CreateWidget` "/Game/Sci-fi_UI_Pack/Widget/UIMenuWidget/MainMenu/WBP_Sci-fi_UI_Pack_BPI_Sci-fi_UI_Pack_Home_StackMenu.WBP_Sci-fi_UI_Pack_BPI_Sci-fi_UI_Pack_Home_StackMenu_C"))
  (bind _output_get (set `self.Home Menu Stack Menu` _returnvalue))
  (`UserWidget.AddToViewport` _output_get 0)
  (`WidgetBlueprintLibrary.SetInputMode_UIOnlyEx` self _output_get)
  (`/Game/Sci-fi_UI_Pack/Widget/UIMenuWidget/MainMenu/WBP_Sci-fi_UI_Pack_BPI_Sci-fi_UI_Pack_Home_StackMenu.Push MainMenuWidget` (`self.Home Menu Stack Menu`) "/Game/Sci-fi_UI_Pack/Widget/UIMenuWidget/GameplayMenu/InventoryMenu/WBP_Sci-fi_UI_Pack_InventoryMenu_.WBP_Sci-fi_UI_Pack_InventoryMenu__C" "Visible" "MouseAndKeyboard"))

(event `self.ReceiveBeginPlay`
  ;[0 0 0 1 45] On begin play Loading Screen intro
  (bind _returnvalue (`|CreateWidget` "/Game/Sci-fi_UI_Pack/Widget/UIMenuWidget/MainMenu/WBP_Sci-fi_UI_Pack_BPI_Sci-fi_UI_Pack_Home_StackMenu.WBP_Sci-fi_UI_Pack_BPI_Sci-fi_UI_Pack_Home_StackMenu_C"))
  (bind _output_get (set `self.Home Menu Stack Menu` _returnvalue))
  (`UserWidget.AddToViewport` _output_get 0)
  (`WidgetBlueprintLibrary.SetInputMode_UIOnlyEx` self (`self.Home Menu Stack Menu`))
  (set `self.bShowMouseCursor` true)
  (if (`self.In Lobby Room Map?`) :!pinned true
    ;[0 0.02593 0.05729 1 40] Check if Player is in  Lobby Room Map, If True Lobby Room Widget
    (`/Game/Sci-fi_UI_Pack/Blueprints/Blueprints_Interface/BPI_Sci-fi_UI_Pack_MultiplayerStackMenuFromOthers.Open Multiplayer Stack Menu From Others`)
    (`/Game/Sci-fi_UI_Pack/Blueprints/Blueprints_Interface/BPI_Sci-fi_UI_Pack_MultiplayerStackMenuFromOthers.Push M Menu` (`self.Lobby `) "Collapsed" (`self.Lobby Room Input Type`))
    (else
      (`/Game/Sci-fi_UI_Pack/Widget/UIMenuWidget/MainMenu/WBP_Sci-fi_UI_Pack_BPI_Sci-fi_UI_Pack_Home_StackMenu.Push MainMenuWidget` _returnvalue "/Game/Sci-fi_UI_Pack/Widget/UIMenuWidget/WBP_Sci-fi_UI_Pack_LoadingScreen.WBP_Sci-fi_UI_Pack_LoadingScreen_C" "Visible" "MouseAndKeyboard")
      (`KismetSystemLibrary.Delay` 5.5)
      (`/Game/Sci-fi_UI_Pack/Widget/UIMenuWidget/MainMenu/WBP_Sci-fi_UI_Pack_BPI_Sci-fi_UI_Pack_Home_StackMenu.Push MainMenuWidget` (`self.Home Menu Stack Menu`) "/Game/Sci-fi_UI_Pack/Widget/UIMenuWidget/WBP_Sci-fi_UI_Pack_StartScreen.WBP_Sci-fi_UI_Pack_StartScreen_C" "Visible" "MouseAndKeyboard"))))

(event `InputAction|Inventory Menu | Key N`
  (params (Key :type "Key Structure"))
  ;[0.0625 0.01759 0 0.833 45] Open Inventory menu
  (:`Pressed`
    (`self.Open Inventory `)))

(event `/Game/Sci-fi_UI_Pack/Blueprints/Blueprints_Interface/BPI_Sci-fi_UI_Pack_Cast_Home_Menu_Stack_Widget.Home Menu Open Gameplay Scene`
  ;[0 0 0 0.5 100] Opening of other menus in Gameplay widget
  ;;[0 0.01667 1 0.458] Begin play for gameplay  scene
  (set `self.Health` (`self.MaxHealth`))
  (set `self.Energy` (`self.MaxEnergy`))
  (bind _returnvalue (`|CreateWidget` "/Game/Sci-fi_UI_Pack/Widget/UIMenuWidget/GameplayMenu/WBP_Sci-fi_UI_Pack_GameplayHUD.WBP_Sci-fi_UI_Pack_GameplayHUD_C"))
  (bind _output_get (set `self.Gameplay HUD Scene` _returnvalue))
  (`UserWidget.AddToViewport` _output_get 0)
  (`WidgetBlueprintLibrary.SetInputMode_GameOnly` self)
  (set `self.bShowMouseCursor` true))

(event `self.Exit Inventory`
  ;[0.0625 0.01759 0 0.833 45] Exit Inventory Menu
  (`Widget.RemoveFromParent` (`self.Home Menu Stack Menu`))
  (`WidgetBlueprintLibrary.SetInputMode_GameOnly` self)
  (set `self.bShowMouseCursor` true))

(event `/Game/Sci-fi_UI_Pack/Blueprints/Blueprints_Interface/BPI_Sci-fi_UI_Pack_Cast_Home_Menu_Stack_Widget.Start Home Menu`
  (params (`Input Device Type` :type "ECommonInputType Enum" :default "MouseAndKeyboard"))
  ;[0 0.03646 0.01499 1 40] Main Menu
  ;;[0 0 0 1 40] Get last game input type
  (bind _output_get (set `self.Input Device Type` `Input Device Type`))
  (`/Game/Sci-fi_UI_Pack/Widget/UIMenuWidget/MainMenu/WBP_Sci-fi_UI_Pack_BPI_Sci-fi_UI_Pack_Home_StackMenu.Push MainMenuWidget` (`self.Home Menu Stack Menu`) (`self.WBP_MainMenu`) "Visible" _output_get))

(event `InputAction|Show Weapon Wheel 1 | Key 3`
  (params (Key :type "Key Structure"))
  ;[0 0 0 0.5 100] Opening of other menus in Gameplay widget
  ;;[0.0625 0.01759 0 0.833] Weapon wheel input actions
  (:`Pressed`
    (`self.Show Weapon Wheel 1`)))

(event `InputAction|Primary Weapon | G`
  (params (Key :type "Key Structure"))
  ;[0 0 0 0.5 100] Opening of other menus in Gameplay widget
  ;;[0 0.1648 0.1823 0.3] Weapon HUD InputAction on Clicked
  (:`Pressed`
    (set `self.WeaponSelected` 0)
    (`self.KeyG`)))

(event `InputAction|Hide Weapon Wheel 1 | Key 4`
  (params (Key :type "Key Structure"))
  ;[0 0 0 0.5 100] Opening of other menus in Gameplay widget
  ;;[0.0625 0.01759 0 0.833] Weapon wheel input actions
  (:`Pressed`
    (`self.Hide Weapon Wheel 1`)))

(event `self.Open Paused Menu`
  (bind _returnvalue (`GameplayStatics.GetGameInstance`))
  ;[0 0.02083 0.02064 0.8 45] Open paused Menu
  (bind _returnvalue_2 (`|CreateWidget` "/Game/Sci-fi_UI_Pack/Widget/UIMenuWidget/MainMenu/WBP_Sci-fi_UI_Pack_BPI_Sci-fi_UI_Pack_Home_StackMenu.WBP_Sci-fi_UI_Pack_BPI_Sci-fi_UI_Pack_Home_StackMenu_C"))
  (bind _output_get (set `self.Home Menu Stack Menu` _returnvalue_2))
  (`UserWidget.AddToViewport` _output_get 0)
  (`WidgetBlueprintLibrary.SetInputMode_UIOnlyEx` self _output_get)
  (if (`KismetSystemLibrary.DoesImplementInterface` _returnvalue "/Game/Sci-fi_UI_Pack/Blueprints/Blueprints_Interface/BPI_Sci-fi_UI_Pack_GameInstance.BPI_Sci-fi_UI_Pack_GameInstance_C")
    (bind _input_type (message `/Game/Sci-fi_UI_Pack/Blueprints/Blueprints_Interface/BPI_Sci-fi_UI_Pack_GameInstance.Get Game Input Type` _returnvalue))
    (`/Game/Sci-fi_UI_Pack/Widget/UIMenuWidget/MainMenu/WBP_Sci-fi_UI_Pack_BPI_Sci-fi_UI_Pack_Home_StackMenu.Push MainMenuWidget` (`self.Home Menu Stack Menu`) "/Game/Sci-fi_UI_Pack/Widget/UIMenuWidget/GameplayMenu/PasuedMenu/WBP_Sci-fi_UI_Pack__PausedMenu.WBP_Sci-fi_UI_Pack__PausedMenu_C" "Collapsed" _input_type)))

(event `InputAction|Granade | J`
  (params (Key :type "Key Structure"))
  ;[0 0 0 0.5 100] Opening of other menus in Gameplay widget
  ;;[0 0.1648 0.1823 0.3] Weapon HUD InputAction on Clicked
  (:`Pressed`
    (set `self.WeaponSelected` 2)
    (`self.KeyJ`)))

(event `InputAction|Show Weapon Wheel 2 | Key 7`
  (params (Key :type "Key Structure"))
  ;[0 0 0 0.5 100] Opening of other menus in Gameplay widget
  ;;[0.0625 0.01759 0 0.833] Weapon wheel input actions
  (:`Pressed`
    (`self.Show Weapon Wheel 2`)))

(event `InputAction|Hide Weapon Wheel 2 | Key 6`
  (params (Key :type "Key Structure"))
  ;[0 0 0 0.5 100] Opening of other menus in Gameplay widget
  ;;[0.0625 0.01759 0 0.833] Weapon wheel input actions
  (:`Pressed`
    (`self.Hide Weapon Wheel 2`)))

(event `InputAction|Open Paused Menu | Key SpaceBar`
  (params (Key :type "Key Structure"))
  ;[0 0.02083 0.02064 0.8 45] Open paused Menu
  (:`Pressed`
    (`self.Open Paused Menu`)))

(event `/Game/Sci-fi_UI_Pack/Blueprints/Blueprints_Interface/BPI_Sci-fi_UI_Pack_Cast_Home_Menu_Stack_Widget.MenuStack`
  (params (Activatable_Widget :type "CommonActivatableWidget Class Reference") (BackgroundVisibility :type "ESlateVisibility Enum" :default "Visible") (`Input Type` :type "ECommonInputType Enum" :default "MouseAndKeyboard"))
  ;[0.002732 0.006049 0.009721 1 50] Home Stack Menu
  (`/Game/Sci-fi_UI_Pack/Widget/UIMenuWidget/MainMenu/WBP_Sci-fi_UI_Pack_BPI_Sci-fi_UI_Pack_Home_StackMenu.Push MainMenuWidget` (`self.Home Menu Stack Menu`) Activatable_Widget BackgroundVisibility `Input Type`))

(event `/Game/Sci-fi_UI_Pack/Blueprints/Blueprints_Interface/BPI_Sci-fi_UI_Pack_PC_Chat.Server_SubmitChat`
  (params (ChatMessage :type Text))
  ;[0 0.009134 0.0185 0.5] For Multiplayer | Connect to server to get name
  ;;[0 0.5607 1 0.15] Server Submit Chat
  (bind _chatpanel (`self.ChatPanel`)
    (:`then`
      (`/Game/Sci-fi_UI_Pack/Widget/UIMenuWidget/MultiplayerWidget/Lobby_UI/Sub_Widget/WBP_Sci-fi_UI_Pack_ChatUI.Update Chat` _chatpanel ChatMessage))
    (:`else`)))

(event `/Game/Sci-fi_UI_Pack/Blueprints/Blueprints_Interface/BPI_Sci-fi_UI_Pack_Cast_Home_Menu_Stack_Widget.Sub_Menu_Stack`
  (params (CommonActivatableWidget :type "CommonActivatableWidget Class Reference") (`Input Type` :type "ECommonInputType Enum" :default "MouseAndKeyboard"))
  ;[0.002732 0.006049 0.009721 1 50] Home Stack Menu
  (`/Game/Sci-fi_UI_Pack/Widget/UIMenuWidget/MainMenu/WBP_Sci-fi_UI_Pack_BPI_Sci-fi_UI_Pack_Home_StackMenu.Push Sub Menu Stack  In` (`self.Home Menu Stack Menu`) CommonActivatableWidget "Visible" `Input Type`))

(event `Key|Enter`
  (params (Key :type "Key Structure"))
  ;[0 0.009134 0.0185 0.5] For Multiplayer | Connect to server to get name
  ;;[0 0.5607 1 0.15] On keyboard enter | get focus
  (:`Pressed`
    (bind _chatpanel (`self.ChatPanel`)
      (:`then`
        (`Widget.SetKeyboardFocus` (`/Game/Sci-fi_UI_Pack/Widget/UIMenuWidget/MultiplayerWidget/Lobby_UI/Sub_Widget/WBP_Sci-fi_UI_Pack_ChatUI.ChatInputBox` _chatpanel)))
      (:`else`))))

(event `Key|Add`
  (params (Key :type "Key Structure"))
  ;[0 0 0 0.5 100] Opening of other menus in Gameplay widget
  ;;[0 0 0 1 30] Increase and Decrease Health Bar
  (:`Pressed`
    (`self.EditHealth` 20.0)))

(event `self.Exit Paused Menu`
  ;[0 0.02083 0.02064 0.8 45] Exit Paused menu
  (`Widget.RemoveFromParent` (`self.Home Menu Stack Menu`))
  (`WidgetBlueprintLibrary.SetInputMode_GameOnly` self)
  (set `self.bShowMouseCursor` true))

(event `EditHealth`
  (params (Amount :type "Float (double-precision)"))
  ;[0 0 0 0.5 100] Opening of other menus in Gameplay widget
  ;;[0 0 0 1 30] Edit Health Increase and Decrease Maximum
  (set `self.Health` (`KismetMathLibrary.FClamp` (+ Amount (`self.Health`)) 0.0 (`self.MaxHealth`))))

(event `Key|Subtract`
  (params (Key :type "Key Structure"))
  ;[0 0 0 0.5 100] Opening of other menus in Gameplay widget
  ;;[0 0 0 1 30] Increase and Decrease Health Bar
  (:`Pressed`
    (`self.EditHealth` -20.0)))

(event `EditEnergy`
  (params (Amount :type "Float (double-precision)"))
  ;[0 0 0 0.5 100] Opening of other menus in Gameplay widget
  ;;[0 0.03646 0.01499 1 30] Edit Health Increase and Decrease Maximum
  (set `self.Energy` (`KismetMathLibrary.FClamp` (+ Amount (`self.Energy`)) 0.0 (`self.MaxEnergy`))))

(event `/Game/Sci-fi_UI_Pack/Blueprints/Blueprints_Interface/BPI_Sci-fi_UI_Pack_Cast_SinglePlayerMenuStack_Widget.Start Single Player Menu`
  ;[0.1406 0 0.024 1 40] Event begin play | Starting from Single Player mainmenu
  (`|ExecutionSequence`
    (:`then_0`
      ;[0.1406 0 0.024 1 45] Single Player MainMenu Variable
      (bind _returnvalue (`|CreateWidget` "/Game/Sci-fi_UI_Pack/Widget/UIMenuWidget/Single_MainMenuUI/HomeMenu/WBP_Sci-fi_UI_Pack_SingleHomeMenu.WBP_Sci-fi_UI_Pack_SingleHomeMenu_C"))
      (set `self.SingleHomeMainMenu` _returnvalue))
    (:`then_1`
      (bind _returnvalue_2 (`|CreateWidget` "/Game/Sci-fi_UI_Pack/Widget/UIMenuWidget/Single_MainMenuUI/WBP_Sci-fi_UI_Pack_SingleMenuStack.WBP_Sci-fi_UI_Pack_SingleMenuStack_C"))
      (bind _output_get (set `self.Single Menu Stack` _returnvalue_2))
      (`UserWidget.AddToViewport` _output_get 0)
      (`/Game/Sci-fi_UI_Pack/Widget/UIMenuWidget/Single_MainMenuUI/WBP_Sci-fi_UI_Pack_SingleMenuStack.Push In Main Menu` _returnvalue_2 "/Game/Sci-fi_UI_Pack/Widget/UIMenuWidget/Single_MainMenuUI/HomeMenu/WBP_Sci-fi_UI_Pack_SingleHomeMenu.WBP_Sci-fi_UI_Pack_SingleHomeMenu_C" "Visible")
      (`WidgetBlueprintLibrary.SetInputMode_UIOnlyEx` self _returnvalue_2)
      (set `self.bShowMouseCursor` true))))

(event `InputAction|SkillHUD_1`
  (params (Key :type "Key Structure"))
  ;[0 0 0 0.5 100] Opening of other menus in Gameplay widget
  ;;[1 0.01332 0 1 78] Skill HUD Input Actions
  (:`Pressed`
    (`self.SkillHUD_1`)))

(event `InputAction|SkillHUD_2`
  (params (Key :type "Key Structure"))
  ;[0 0 0 0.5 100] Opening of other menus in Gameplay widget
  ;;[1 0.01332 0 1 78] Skill HUD Input Actions
  (:`Pressed`
    (`self.SkillHUD_2`)))

(event `InputAction|Increase Energy | Key 1`
  (params (Key :type "Key Structure"))
  ;[0 0 0 0.5 100] Opening of other menus in Gameplay widget
  ;;[0 0.03646 0.01499 1 30] Increase and Decrease Energy Bar
  (:`Pressed`
    (`self.EditEnergy` 20.0)))

(event `InputAction|SkillHUD_3`
  (params (Key :type "Key Structure"))
  ;[0 0 0 0.5 100] Opening of other menus in Gameplay widget
  ;;[1 0.01332 0 1 78] Skill HUD Input Actions
  (:`Pressed`
    (`self.SkillHUD_3`)))

(event `InputAction|SkillHUD_4`
  (params (Key :type "Key Structure"))
  ;[0 0 0 0.5 100] Opening of other menus in Gameplay widget
  ;;[1 0.01332 0 1 78] Skill HUD Input Actions
  (:`Pressed`
    (`self.SkillHUD_4`)))

(event `InputAction|Decrease Energy | Key 2`
  (params (Key :type "Key Structure"))
  ;[0 0 0 0.5 100] Opening of other menus in Gameplay widget
  ;;[0 0.03646 0.01499 1 30] Increase and Decrease Energy Bar
  (:`Pressed`
    (`self.EditEnergy` -20.0)))

(event `/Game/Sci-fi_UI_Pack/Blueprints/Blueprints_Interface/BPI_Sci-fi_UI_Pack_Cast_SinglePlayerMenuStack_Widget.SinglePlayer_Sub_Menu_Stack`
  (params (CommonActivatableWidget :type "CommonActivatableWidget Class Reference"))
  ;[0 0.02 0.01436 1 45] Single Player Stack Menu
  (`/Game/Sci-fi_UI_Pack/Widget/UIMenuWidget/Single_MainMenuUI/WBP_Sci-fi_UI_Pack_SingleMenuStack.Push In Sub Menu` (`self.Single Menu Stack`) CommonActivatableWidget))

(event `/Game/Sci-fi_UI_Pack/Blueprints/Blueprints_Interface/BPI_Sci-fi_UI_Pack_Cast_SinglePlayerMenuStack_Widget.SinglePlayer_MenuStack`
  (params (Activatable_Widget :type "CommonActivatableWidget Class Reference") (BackgroundVisibility :type "ESlateVisibility Enum" :default "Visible"))
  ;[0 0.02 0.01436 1 45] Single Player Stack Menu
  (`/Game/Sci-fi_UI_Pack/Widget/UIMenuWidget/Single_MainMenuUI/WBP_Sci-fi_UI_Pack_SingleMenuStack.Push In Main Menu` (`self.Single Menu Stack`) Activatable_Widget BackgroundVisibility))

(event `/Game/Sci-fi_UI_Pack/Blueprints/Blueprints_Interface/BPI_Sci-fi_UI_Pack_Cast_Home_Menu_Stack_Widget.Set CharacterMenu_SpawnTransform`
  (params (CharacterWeaponMenu_SpawnTransform_ :type "Transform Structure"))
  ;[0 0.02 0.01436 1 45] Set Menu Character Weapon World Transform
  (set `self.CharacterMenu_SpawnTransform` CharacterWeaponMenu_SpawnTransform_))

(event `/Game/Sci-fi_UI_Pack/Blueprints/Blueprints_Interface/BPI_Sci-fi_UI_Pack_Cast_Home_Menu_Stack_Widget.Set WeaponMenu_SpawnTransform`
  (params (CharacterWeaponMenu_SpawnTransform_ :type "Transform Structure"))
  ;[0 0.02 0.01436 1 45] Set Menu Character Weapon World Transform
  (set `self.WeaponMenu_SpawnTransform` CharacterWeaponMenu_SpawnTransform_))

(event `/Game/Sci-fi_UI_Pack/Blueprints/Blueprints_Interface/BPI_Sci-fi_UI_Pack_Cast_Home_Menu_Stack_Widget.Set In Lobby Room Map?`
  (params (`In Lobby Room Map?` :type Boolean) (`Input Type` :type "ECommonInputType Enum" :default "MouseAndKeyboard"))
  ;[0.9294 1 0.6157 1 45] Set In Lobby Room Map? to True to avoid showing Start Screen Again
  (set `self.In Lobby Room Map?` `In Lobby Room Map?`)
  (set `self.Lobby Room Input Type` `Input Type`))

(event `/Game/Sci-fi_UI_Pack/Blueprints/Blueprints_Interface/BPI_Sci-fi_UI_Pack_MultiplayerStackMenuFromOthers.Open Multiplayer Stack Menu From Others`
  ;[0.03689 0.000607 0 1 45] Open Multiplayer Stack Menu from other / Open From Character Options
  (bind _returnvalue (`|CreateWidget` "/Game/Sci-fi_UI_Pack/Widget/UIMenuWidget/MultiplayerWidget/WBP_Sci-fi_UI_Pack_MultiplayerStackMenuFromOthers.WBP_Sci-fi_UI_Pack_MultiplayerStackMenuFromOthers_C"))
  (bind _output_get (set `self.MultiplayerStackMenuFromOthers` _returnvalue))
  (`UserWidget.AddToViewport` _output_get 0)
  (`WidgetBlueprintLibrary.SetInputMode_UIOnlyEx` self _output_get)
  (set `self.bShowMouseCursor` true))

(event `/Game/Sci-fi_UI_Pack/Blueprints/Blueprints_Interface/BPI_Sci-fi_UI_Pack_MultiplayerStackMenuFromOthers.Push M Menu`
  (params (`Common Activateable Widget` :type "CommonActivatableWidget Class Reference") (`Background Visibility` :type "ESlateVisibility Enum" :default "Visible") (`Input Type` :type "ECommonInputType Enum" :default "MouseAndKeyboard"))
  ;[0.03689 0.000607 0 1 45] Push multiplayer menu and sub menu
  (`/Game/Sci-fi_UI_Pack/Widget/UIMenuWidget/MultiplayerWidget/WBP_Sci-fi_UI_Pack_MultiplayerStackMenuFromOthers.Push M_Menu` (`self.MultiplayerStackMenuFromOthers`) `Common Activateable Widget` `Background Visibility` `Input Type`))

(event `/Game/Sci-fi_UI_Pack/Blueprints/Blueprints_Interface/BPI_Sci-fi_UI_Pack_MultiplayerStackMenuFromOthers.Remove Multiplayer Stack Menu, Open Main Menu`
  ;[0.03689 0.000607 0 1 45] Event Remove Multiplayer Stack menu widget, open Main menus from Home
  (`Widget.RemoveFromParent` (`self.MultiplayerStackMenuFromOthers`)))

(event `/Game/Sci-fi_UI_Pack/Blueprints/Blueprints_Interface/BPI_Sci-fi_UI_Pack_MultiplayerStackMenuFromOthers.Push M Sub Menu`
  (params (`Common Activateable Widget` :type "CommonActivatableWidget Class Reference"))
  ;[0.03689 0.000607 0 1 45] Push multiplayer menu and sub menu
  (`/Game/Sci-fi_UI_Pack/Widget/UIMenuWidget/MultiplayerWidget/WBP_Sci-fi_UI_Pack_MultiplayerStackMenuFromOthers.Push Sub Menu Stack  In` (`self.MultiplayerStackMenuFromOthers`) `Common Activateable Widget`))

(fn `Get CharacterMenu_SpawnTransform`
  (returns (CharacterWeaponMenu_SpawnTransform :type "Transform Structure"))
  (return (`self.CharacterMenu_SpawnTransform`)))

(fn `Get WeaponMenu_SpawnTransform`
  (returns (CharacterWeaponMenu_SpawnTransform :type "Transform Structure"))
  (return (`self.WeaponMenu_SpawnTransform`)))

(fn `GetEnergy`
  (returns (Result :type "Float (double-precision)"))
  (return (`self.Energy`)))

(fn `GetEnergyAsRatio`
  (returns (Result :type "Float (double-precision)"))
  (bind _result (`self.GetEnergy`))
  (return (/ _result (`self.MaxEnergy`))))

(fn `GetHealth`
  (returns (Result :type "Float (double-precision)"))
  (return (`self.Health`)))

(fn `GetHealthAsRatio`
  (returns (Result :type "Float (double-precision)"))
  (bind _result (`self.GetHealth`))
  (return (/ _result (`self.MaxHealth`))))

(fn `Home Menu ConfirmationDialogBox`
  (params (ActivateableWIdget :type "CommonActivatableWidget Class Reference") (Title_Text :type Text) (Note :type Text) (PromptOwner :type "CommonActivatableWidget Object Reference"))
  (returns (ReturnValue :type "/Game/Sci-fi_UI_Pack/Widget/UIMenuWidget/QuitGame/WBP_Sci-fi_UI_Pack_QuitGame_Widget Object Reference"))
  (bind _returnvalue (`/Game/Sci-fi_UI_Pack/Widget/UIMenuWidget/MainMenu/WBP_Sci-fi_UI_Pack_BPI_Sci-fi_UI_Pack_Home_StackMenu.Push_ConfirmationDialogBox_In_` (`self.Home Menu Stack Menu`) Title_Text ActivateableWIdget Note PromptOwner))
  (return _returnvalue))

(fn `Open Confirmation Dialogue Menu`
  (params (`Title Text` :type Text) (`Activateable Widget` :type "CommonActivatableWidget Class Reference") (`Note Prompt` :type Text) (`Prompt Owner` :type "CommonActivatableWidget Object Reference"))
  (returns (`Return Value` :type "/Game/Sci-fi_UI_Pack/Widget/UIMenuWidget/QuitGame/WBP_Sci-fi_UI_Pack_QuitGame_Widget Object Reference"))
  (bind _returnvalue (`/Game/Sci-fi_UI_Pack/Widget/UIMenuWidget/MultiplayerWidget/WBP_Sci-fi_UI_Pack_MultiplayerStackMenuFromOthers.Push_ConfirmationDialogBox_In_` (`self.MultiplayerStackMenuFromOthers`) `Title Text` `Activateable Widget` `Note Prompt` `Prompt Owner`))
  (return _returnvalue))

(fn `Show_NotificationPrompt`
  (params (ActivateableWIdget :type "CommonActivatableWidget Class Reference") (`Player's Name` :type Text) (Note :type Text) (`Owning Player` :type "CommonActivatableWidget Object Reference"))
  (returns (ReturnValue :type "/Game/Sci-fi_UI_Pack/Widget/UIMenuWidget/PopUp_Menu/WBP_Sci-fi_UI_Pack_Notification Object Reference"))
  (bind _returnvalue (`/Game/Sci-fi_UI_Pack/Widget/UIMenuWidget/MainMenu/WBP_Sci-fi_UI_Pack_BPI_Sci-fi_UI_Pack_Home_StackMenu.Push_NotificationPrompt_In` (`self.Home Menu Stack Menu`) ActivateableWIdget `Player's Name` Note `Owning Player`))
  (return _returnvalue))

(fn `Single Player ConfirmationDialogBox`
  (params (Title_Text :type Text) (ActivateableWIdget :type "CommonActivatableWidget Class Reference") (`Note Prompt` :type Text) (PromptOwner :type "CommonActivatableWidget Object Reference"))
  (returns (ReturnValue :type "/Game/Sci-fi_UI_Pack/Widget/UIMenuWidget/QuitGame/WBP_Sci-fi_UI_Pack_QuitGame_Widget Object Reference"))
  (bind _returnvalue (`/Game/Sci-fi_UI_Pack/Widget/UIMenuWidget/Single_MainMenuUI/WBP_Sci-fi_UI_Pack_SingleMenuStack.Push Confirmation Dialog Box In ` (`self.Single Menu Stack`) Title_Text ActivateableWIdget `Note Prompt` PromptOwner))
  (return _returnvalue))

(fn `UserConstructionScript`)