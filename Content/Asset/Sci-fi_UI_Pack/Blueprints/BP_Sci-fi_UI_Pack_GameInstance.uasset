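; Game Instance for the Sci-fi UI Pack that serves as the central hub for graphics, audio, gameplay and language settings, and tracks the input type.
; Graphics options go through GameUserSettings, while the other settings persist in a lazily loaded or created SaveGame.
; Volumes apply through sound mix class overrides, and mouse sensitivity and Y inversion by rebuilding axis mappings.
; Init reapplies saved audio after a short delay and restores the saved culture.
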(event `self.ReceiveInit`
  (bind _language (`/Game/Sci-fi_UI_Pack/Blueprints/SaveFiles/BP_Sci-fi_UI_Pack_UI_Settings_SaveGame.Language` (`self.BP Sci-fi UI Pack UI Settings Save Game`)))
  ;[0.03689 0.000607 0 1 45] init Reload Audio settings
  (bind _bp_sci_fi_ui_pack_ui_settings_save_game (`self.Load Settings`))
  (`KismetSystemLibrary.Delay` 0.2)
  (message `/Game/Sci-fi_UI_Pack/Blueprints/Blueprints_Interface/BPI_Sci-fi_UI_Pack_GameInstance.Save Audio Settings` self (`/Game/Sci-fi_UI_Pack/Blueprints/SaveFiles/BP_Sci-fi_UI_Pack_UI_Settings_SaveGame.MasterVolume` _bp_sci_fi_ui_pack_ui_settings_save_game) (`/Game/Sci-fi_UI_Pack/Blueprints/SaveFiles/BP_Sci-fi_UI_Pack_UI_Settings_SaveGame.SfxVolume` _bp_sci_fi_ui_pack_ui_settings_save_game) (`/Game/Sci-fi_UI_Pack/Blueprints/SaveFiles/BP_Sci-fi_UI_Pack_UI_Settings_SaveGame.MusicVolume` _bp_sci_fi_ui_pack_ui_settings_save_game) (`/Game/Sci-fi_UI_Pack/Blueprints/SaveFiles/BP_Sci-fi_UI_Pack_UI_Settings_SaveGame.DialogueVolume` _bp_sci_fi_ui_pack_ui_settings_save_game))
  (if (> (`KismetArrayLibrary.Array_Find` (`KismetInternationalizationLibrary.GetLocalizedCultures` true) _language) 0)
    (`KismetInternationalizationLibrary.SetCurrentCulture` _language)))

(event `/Game/Sci-fi_UI_Pack/Blueprints/Blueprints_Interface/BPI_Sci-fi_UI_Pack_GameInstance.Apply Graphic Settings`
  (params (`Anti Aliasing Quality` :type Integer) (`Texture Quality` :type Integer) (`Post Process Quality` :type Integer) (`View Distance Quality` :type Integer) (`Shading Quality` :type Integer) (`Reflections Quality` :type Integer) (`Shadow Quality` :type Integer) (`Global Illumination Quality` :type Integer) (Vsync :type Boolean))
  ;[0.02604 0.000602 0 0.542 45] BPI Apply Graphic Settings
  (`self.Set Game Settings` `Anti Aliasing Quality` `Texture Quality` `Post Process Quality` `View Distance Quality` `Shading Quality` `Reflections Quality` `Shadow Quality` `Global Illumination Quality` Vsync))

(event `Set Game Settings`
  (params (`Anti Aliasing Value` :type Integer) (`Texture Qua Value` :type Integer) (`Post Processing Qua Value` :type Integer) (`View Distance Qua Value` :type Integer) (`Shading Qua Value` :type Integer) (`Reflection Qua Value` :type Integer) (`Shadow Qua Value` :type Integer) (`G_Illumination Qua Value` :type Integer) (VerticalSync :type Boolean))
  ;[0.02604 0.000602 0 0.542 45] Set Game Settings
  (bind _returnvalue (`GameUserSettings.GetGameUserSettings`))
  (`GameUserSettings.SetAntiAliasingQuality` _returnvalue `Anti Aliasing Value`)
  (`GameUserSettings.SetShadingQuality` _returnvalue `Shading Qua Value`)
  (`GameUserSettings.SetTextureQuality` _returnvalue `Texture Qua Value`)
  (`GameUserSettings.SetPostProcessingQuality` _returnvalue `Post Processing Qua Value`)
  (`GameUserSettings.SetViewDistanceQuality` _returnvalue `View Distance Qua Value`)
  (`GameUserSettings.SetReflectionQuality` _returnvalue `Reflection Qua Value`)
  (`GameUserSettings.SetGlobalIlluminationQuality` _returnvalue `G_Illumination Qua Value`)
  (`GameUserSettings.SetShadowQuality` _returnvalue `Shadow Qua Value`)
  (`GameUserSettings.SetVSyncEnabled` _returnvalue VerticalSync))

(event `/Game/Sci-fi_UI_Pack/Blueprints/Blueprints_Interface/BPI_Sci-fi_UI_Pack_GameInstance.Apply Resolution Settings`
  ;[9.9e-05 0.0137 0 0.8 45] Apply Resolution Settings
  (bind _returnvalue (`GameUserSettings.GetGameUserSettings`))
  (`GameUserSettings.ApplyResolutionSettings` _returnvalue false))

(event `/Game/Sci-fi_UI_Pack/Blueprints/Blueprints_Interface/BPI_Sci-fi_UI_Pack_GameInstance.Save Audio Settings`
  (params (`Master Volume` :type "Float (double-precision)") (`Sfx Volume` :type "Float (double-precision)") (`Music Volume` :type "Float (double-precision)") (`Dialogue Volume` :type "Float (double-precision)"))
  (bind _bp_sci_fi_ui_pack_ui_settings_save_game (`self.BP Sci-fi UI Pack UI Settings Save Game`))
  ;[0.02604 0.000602 0 0.542 45] Save Audio Settings
  (`GameplayStatics.SetSoundMixClassOverride` "/Game/Sci-fi_UI_Pack/Audio/SoundClass/SCM_Sci-fi_UI_Pack__MasterMix.SCM_Sci-fi_UI_Pack__MasterMix" "/Game/Sci-fi_UI_Pack/Audio/SoundClass/SC_Sci-fi_UI_Pack_Master.SC_Sci-fi_UI_Pack_Master" `Master Volume` 1.0 0.0)
  (`GameplayStatics.SetSoundMixClassOverride` "/Game/Sci-fi_UI_Pack/Audio/SoundClass/SCM_Sci-fi_UI_Pack__FX_Mix.SCM_Sci-fi_UI_Pack__FX_Mix" "/Game/Sci-fi_UI_Pack/Audio/SoundClass/SC_Sci-fi_UI_Pack_FX.SC_Sci-fi_UI_Pack_FX" `Sfx Volume` 1.0 0.0)
  (`GameplayStatics.SetSoundMixClassOverride` "/Game/Sci-fi_UI_Pack/Audio/SoundClass/SCM_Sci-fi_UI_Pack__MusicMix.SCM_Sci-fi_UI_Pack__MusicMix" "/Game/Sci-fi_UI_Pack/Audio/SoundClass/SC_Sci-fi_UI_Pack_Music.SC_Sci-fi_UI_Pack_Music" `Music Volume` 1.0 0.0)
  (`GameplayStatics.SetSoundMixClassOverride` "/Game/Sci-fi_UI_Pack/Audio/SoundClass/SCM_Sci-fi_UI_Pack__DialogueMix.SCM_Sci-fi_UI_Pack__DialogueMix" "/Game/Sci-fi_UI_Pack/Audio/SoundClass/SC_Sci-fi_UI_Pack_Dialogue.SC_Sci-fi_UI_Pack_Dialogue" `Dialogue Volume` 1.0 0.0)
  (`self.Load Settings`)
  (set `/Game/Sci-fi_UI_Pack/Blueprints/SaveFiles/BP_Sci-fi_UI_Pack_UI_Settings_SaveGame.MasterVolume` `Master Volume` _bp_sci_fi_ui_pack_ui_settings_save_game)
  (set `/Game/Sci-fi_UI_Pack/Blueprints/SaveFiles/BP_Sci-fi_UI_Pack_UI_Settings_SaveGame.MusicVolume` `Music Volume` _bp_sci_fi_ui_pack_ui_settings_save_game)
  (set `/Game/Sci-fi_UI_Pack/Blueprints/SaveFiles/BP_Sci-fi_UI_Pack_UI_Settings_SaveGame.SfxVolume` `Sfx Volume` _bp_sci_fi_ui_pack_ui_settings_save_game)
  (set `/Game/Sci-fi_UI_Pack/Blueprints/SaveFiles/BP_Sci-fi_UI_Pack_UI_Settings_SaveGame.DialogueVolume` `Dialogue Volume` _bp_sci_fi_ui_pack_ui_settings_save_game)
  (`self.SaveSettings`))

(event `/Game/Sci-fi_UI_Pack/Blueprints/Blueprints_Interface/BPI_Sci-fi_UI_Pack_GameInstance.Save Settings`
  ;[9.9e-05 0.0137 0 0.8 45] Save Settings
  (bind _returnvalue (`GameUserSettings.GetGameUserSettings`))
  (`GameUserSettings.SaveSettings` _returnvalue))

(event `/Game/Sci-fi_UI_Pack/Blueprints/Blueprints_Interface/BPI_Sci-fi_UI_Pack_GameInstance.Apply Settings`
  ;[9.9e-05 0.0137 0 0.8 45] Apply settings
  (bind _returnvalue (`GameUserSettings.GetGameUserSettings`))
  (`GameUserSettings.ApplySettings` _returnvalue false))

(event `/Game/Sci-fi_UI_Pack/Blueprints/Blueprints_Interface/BPI_Sci-fi_UI_Pack_GameInstance.SaveGameplaySettings`
  (params (DifficultyLevel :type Integer) (InvertMouseY_Axis :type Boolean) (MouseY_Sensitivity :type "Float (double-precision)") (MouseX_Sensitivity :type "Float (double-precision)"))
  (bind _bp_sci_fi_ui_pack_ui_settings_save_game (`self.BP Sci-fi UI Pack UI Settings Save Game`))
  ;[0.02604 0.000602 0 0.542 45] Save Gameplay Settings
  (`self.Load Settings`)
  (set `/Game/Sci-fi_UI_Pack/Blueprints/SaveFiles/BP_Sci-fi_UI_Pack_UI_Settings_SaveGame.Difficulty` DifficultyLevel _bp_sci_fi_ui_pack_ui_settings_save_game)
  (`self.Mouse Y Update` InvertMouseY_Axis MouseY_Sensitivity _bp_sci_fi_ui_pack_ui_settings_save_game)
  (`self.Mouse X Update` MouseX_Sensitivity _bp_sci_fi_ui_pack_ui_settings_save_game)
  (`self.SaveSettings`))

(event `/Game/Sci-fi_UI_Pack/Blueprints/Blueprints_Interface/BPI_Sci-fi_UI_Pack_GameInstance.SaveLanguageSettings`
  (params (Language :type String))
  ;[0.0625 0.01759 0 0.833 45] Save Language Settings
  (`self.Load Settings`)
  (set `/Game/Sci-fi_UI_Pack/Blueprints/SaveFiles/BP_Sci-fi_UI_Pack_UI_Settings_SaveGame.Language` Language (`self.BP Sci-fi UI Pack UI Settings Save Game`))
  (`self.SaveSettings`))

(event `/Game/Sci-fi_UI_Pack/Blueprints/Blueprints_Interface/BPI_Sci-fi_UI_Pack_GameInstance.Set Game Input Type`
  (params (`Input Type` :type "ECommonInputType Enum" :default "MouseAndKeyboard"))
  ;[1 0 0 1 45] Set last game input type
  (set `self.Input Type ` `Input Type`))

(fn `Get Game Input Type`
  (returns (`Input Type` :type "ECommonInputType Enum"))
  (return (`self.Input Type `)))

(fn `Get Settings`
  (returns (Settings :type "/Game/Sci-fi_UI_Pack/Blueprints/SaveFiles/BP_Sci-fi_UI_Pack_UI_Settings_SaveGame Object Reference"))
  (bind _bp_sci_fi_ui_pack_ui_settings_save_game (`self.Load Settings`))
  (return _bp_sci_fi_ui_pack_ui_settings_save_game))

(fn `Mouse X Update`
  (params (`Mouse X Sensitivity` :type "Float (double-precision)") (BP_Settings_SaveGame :type "/Game/Sci-fi_UI_Pack/Blueprints/SaveFiles/BP_Sci-fi_UI_Pack_UI_Settings_SaveGame Object Reference"))
  (locals (`Turn Right / Left Mouse` :type "Array of InputAxisKeyMapping Structure"))
  (bind _returnvalue (`InputSettings.GetInputSettings`))
  (bind _output_get (set `/Game/Sci-fi_UI_Pack/Blueprints/SaveFiles/BP_Sci-fi_UI_Pack_UI_Settings_SaveGame.Mouse X Sensitivity` `Mouse X Sensitivity` BP_Settings_SaveGame))
  (bind _output_get_2 (set `local.Turn Right / Left Mouse` (`InputSettings.GetAxisMappingByName` _returnvalue "Turn Right / Left Mouse")))
  (for _array_element _output_get_2
    (`InputSettings.RemoveAxisMapping` _returnvalue _array_element true)
    (bind _structout (setmembers `InputAxisKeyMapping` :`StructRef` _array_element :`Scale` (`KismetMathLibrary.FClamp` (* _output_get 2.0) 0.1 2.0)))
    (`InputSettings.AddAxisMapping` _returnvalue _structout true)))

(fn `Mouse Y Update`
  (params (InvertMouseY_Axis :type Boolean) (`Mouse Y Sensitivity` :type "Float (double-precision)") (BP_Settings_SaveGame :type "/Game/Sci-fi_UI_Pack/Blueprints/SaveFiles/BP_Sci-fi_UI_Pack_UI_Settings_SaveGame Object Reference"))
  (locals (`Look Up / Down Mouse` :type "Array of InputAxisKeyMapping Structure"))
  (bind _returnvalue (`InputSettings.GetInputSettings`))
  (bind _output_get (set `/Game/Sci-fi_UI_Pack/Blueprints/SaveFiles/BP_Sci-fi_UI_Pack_UI_Settings_SaveGame.InvertMouseY_Axis` InvertMouseY_Axis BP_Settings_SaveGame))
  (bind _output_get_2 (set `/Game/Sci-fi_UI_Pack/Blueprints/SaveFiles/BP_Sci-fi_UI_Pack_UI_Settings_SaveGame.Mouse Y Sensitivity` `Mouse Y Sensitivity` BP_Settings_SaveGame))
  (bind _output_get_3 (set `local.Look Up / Down Mouse` (`InputSettings.GetAxisMappingByName` (`InputSettings.GetInputSettings`) "Look Up / Down Mouse")))
  (for _array_element _output_get_3
    (`InputSettings.RemoveAxisMapping` _returnvalue _array_element true)
    (bind _structout (setmembers `InputAxisKeyMapping` :`StructRef` _array_element :`Scale` (* (`KismetMathLibrary.FClamp` (* _output_get_2 2.0) 0.1 2.0) (`KismetMathLibrary.SelectFloat` 1.0 -1.0 _output_get))))
    (`InputSettings.AddAxisMapping` _returnvalue _structout true)))

(fn `SaveSettings`
  (`GameplayStatics.SaveGameToSlot` (`self.BP Sci-fi UI Pack UI Settings Save Game`) (`self.Settings Save Slot`)))