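; BP_ProjectPlayer is the player Blueprint that opens and closes the skill tree and skill choice screens from input actions.
; Each key toggles its widget, switching cursor visibility and input mode between game-only and game-and-UI.
; Either menu opens only while the other is closed, and each widget receives a reference to the player.
; The skill tree's SkillCost text is filled from the player's skill points on open.
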(event `self.ReceiveBeginPlay`)

(event `EnhancedInput|/Game/Inputs/IA_SkillTree`
  (params (ActionValue :type Boolean) (ElapsedSeconds :type "Float (double-precision)") (TriggeredSeconds :type "Float (double-precision)") (InputAction :type "InputAction Object Reference" :default "/Game/Inputs/IA_SkillTree.IA_SkillTree"))
  (bind _returnvalue (`GameplayStatics.GetPlayerController` 0))
  (bind _returnvalue_2 (`GameplayStatics.GetPlayerController` 0))
  (bind _skill_tree_widget (`self.Skill Tree Widget`))
  (:`Started`
    (`self.Skill Choice Widget`
      (:`then`)
      (:`else`
        (`self.Skill Tree Widget`
          (:`then`
            (`Widget.RemoveFromParent` (`self.Skill Tree Widget`))
            (set `self.Skill Tree Widget` null)
            (set `PlayerController.bShowMouseCursor` false _returnvalue)
            (`WidgetBlueprintLibrary.SetInputMode_GameOnly` _returnvalue))
          (:`else`
            (bind _returnvalue_3 (`|CreateWidget` "/Game/BluePrints/UI/WB_SkillTree.WB_SkillTree_C"))
            (bind _output_get (set `self.Skill Tree Widget` _returnvalue_3))
            (`UserWidget.AddToViewport` _output_get 0)
            (set `PlayerController.bShowMouseCursor` true _returnvalue_2)
            (`WidgetBlueprintLibrary.SetInputMode_GameAndUIEx` _returnvalue_2 null)
            (bind _output_get_2 (set `/Game/BluePrints/UI/WB_SkillTree.Player` self _skill_tree_widget))
            (set `TextBlock.Text` (`KismetTextLibrary.Conv_IntToText` (`self.GetSkillPoint` _output_get_2)) (`/Game/BluePrints/UI/WB_SkillTree.SkillCost` _skill_tree_widget))))))))

(event `EnhancedInput|/Game/Inputs/IA_SkillChoice`
  (params (ActionValue :type Boolean) (ElapsedSeconds :type "Float (double-precision)") (TriggeredSeconds :type "Float (double-precision)") (InputAction :type "InputAction Object Reference" :default "/Game/Inputs/IA_SkillChoice.IA_SkillChoice"))
  (bind _returnvalue (`GameplayStatics.GetPlayerController` 0))
  (bind _returnvalue_2 (`GameplayStatics.GetPlayerController` 0))
  (:`Started`
    (`self.Skill Tree Widget`
      (:`then`)
      (:`else`
        (`self.Skill Choice Widget`
          (:`then`
            (`Widget.RemoveFromParent` (`self.Skill Choice Widget`))
            (set `self.Skill Choice Widget` null)
            (set `PlayerController.bShowMouseCursor` false _returnvalue)
            (`WidgetBlueprintLibrary.SetInputMode_GameOnly` _returnvalue))
          (:`else`
            (bind _returnvalue_3 (`|CreateWidget` "/Game/BluePrints/UI/WB_SkillChoicePanel.WB_SkillChoicePanel_C"))
            (bind _output_get (set `self.Skill Choice Widget` _returnvalue_3))
            (`UserWidget.AddToViewport` _output_get 0)
            (set `/Game/BluePrints/UI/WB_SkillChoicePanel.Player` self (`self.Skill Choice Widget`))
            (set `PlayerController.bShowMouseCursor` true _returnvalue_2)
            (`WidgetBlueprintLibrary.SetInputMode_GameAndUIEx` _returnvalue_2 null)))))))

(fn `UserConstructionScript`)